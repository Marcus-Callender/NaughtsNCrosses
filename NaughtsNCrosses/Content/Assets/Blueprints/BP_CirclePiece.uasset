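; BP_CirclePiece is a clickable circle on a game board that takes the current colour when claimed.
; Its construction script caches the first BP_GameBoard in the level and prints an error if none is valid.
; On click, if the board allows it and the piece's colour is still the initial enum value, it copies the board's current colour and tints its mesh material red or cyan.
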(event OnClicked(SM_BaseCircle)
  (params (TouchedComponent :type Primitive%20Component%20Object%20Reference) (ButtonPressed :type Key%20Structure :default "AnyKey"))
  (if (and (Variables|/Game/Assets/Blueprints/BP_GameBoard.BP_GameBoard_C|Getm_canClick (Variables|Default|Getm_pGameBoard)) (Utilities|Enum|Equal(Enum) (Variables|Default|Getm_myColour) "NewEnumerator0"))
    (Variables|Default|Setm_myColour (Variables|/Game/Assets/Blueprints/BP_GameBoard.BP_GameBoard_C|Getm_currentColour (Variables|Default|Getm_pGameBoard)))
    (if (Utilities|Enum|Equal(Enum) (Variables|Default|Getm_myColour) "NewEnumerator1")
      (Rendering|Material|SetVectorParameterValueonMaterials (Variables|Default|GetSM_BaseCircle) "Colour" "1.000000, 0, 0")
      (elif (Utilities|Enum|Equal(Enum) (Variables|Default|Getm_myColour) "NewEnumerator2")
        (Rendering|Material|SetVectorParameterValueonMaterials (Variables|Default|GetSM_BaseCircle) "Colour" "0.000000,1.000000,1.000000")))))

(event EventBeginPlay)

(event Collision|EventActorBeginOverlap
  (params (OtherActor :type Actor%20Object%20Reference)))

(event EventTick
  (params (DeltaSeconds :type Float%20%28single-precision%29)))

(fn ConstructionScript
  (bind _outactors (Actor|GetAllActorsOfClass "/Game/Assets/Blueprints/BP_GameBoard.BP_GameBoard_C"))
  (bind _output_get (Variables|Default|Setm_pGameBoard (Utilities|Array|Get(acopy) _outactors)))
  (Utilities|IsValid _output_get
    (:Is%20Not%20Valid
      (Development|PrintString "Refrence not Valid"))))