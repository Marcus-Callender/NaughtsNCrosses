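; BP_GameBoard runs a two-colour, line-matching board game, handling turns, win detection and reset.
; PieceClicked locks input, waits, then runs CheckVictory, either swapping colour or announcing the winner and resetting.
; Win checks start from BP_CirclePiece actors and chain neighbour links for five matching pieces.
; Both horizontal and vertical checks follow bottom links, leaving the right-link helper unused, and ResetGame leaves clicking disabled.
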(event Custom|PieceClicked
  (Variables|Default|Setm_canClick false)
  (Utilities|FlowControl|Delay 0.75)
  (Utilities|CheckVictory
    (:Out
      (if (Variables|Default|Getm_gameWon)
        (Development|PrintText (Utilities|Text|ToText(String) (Utilities|String|EnumtoString (Variables|Default|Getm_currentColour))) true true "(R=0.000000,G=0.660000,B=1.000000,A=1.000000)" 5.0)
        (Utilities|FlowControl|Delay 3.0)
        (Utilities|ResetGame)
        (else
          (if (Utilities|Enum|Equal(Enum) (Variables|Default|Getm_currentColour) "NewEnumerator1")
            (Variables|Default|Setm_currentColour "NewEnumerator2")
            (else
              (Variables|Default|Setm_currentColour "NewEnumerator1")))
          (Variables|Default|Setm_canClick true))))))

(event EventBeginPlay)

(event Collision|EventActorBeginOverlap
  (params (OtherActor :type Actor%20Object%20Reference)))

(event EventTick
  (params (DeltaSeconds :type Float%20%28single-precision%29)))

(fn ConstructionScript)